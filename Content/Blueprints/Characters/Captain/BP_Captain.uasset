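; BP_Captain is the Captain character Blueprint, with a combat component, an attack hitbox and debug text readouts.
; Its only active logic runs on Tick, writing current health from CombatComponent, converted to a byte, into DebugHP.
; Tick also sets HitBoxActive to show whether the AttackHitBox collision is Query Only.
; BeginPlay and the construction script are empty.
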(event EventBeginPlay)

(event Collision|EventActorBeginOverlap
  (params (OtherActor :type Actor%20Object%20Reference)))

(event EventTick
  (params (DeltaSeconds :type Float%20%28single-precision%29))
  (Rendering|Components|TextRender|SetText (Variables|Default|GetDebugHP) (Utilities|Text|ToText(String) (Math|Conversions|ToByte(Integer) (Variables|/Script/ActionPlatformer2D3D.APCombatComponent|GetCurrentHealth (Variables|Default|GetCombatComponent)))))
  (Rendering|Components|TextRender|SetText (Variables|Default|GetHitBoxActive) (Utilities|Text|ToText(Boolean) (Utilities|Enum|Equal(Enum) "QueryOnly" (Collision|GetCollisionEnabled (Variables|Default|GetAttackHitBox))))))

(fn ConstructionScript)