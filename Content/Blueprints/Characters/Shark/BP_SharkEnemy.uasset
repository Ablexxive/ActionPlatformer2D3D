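; BP_SharkEnemy is a shark enemy that targets the captain when they enter its aggro range.
; An AggroSphere overlap with a BP_Captain passes that actor to the AIC_Shark controller through SetAttackTarget.
; For debugging, the sphere is made visible at BeginPlay, and Tick updates text showing current health from CombatComponent and whether AttackHitBox collision is query-only.
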(event OnComponentBeginOverlap(AggroSphere)
  (params (OverlappedComponent :type Primitive%20Component%20Object%20Reference) (OtherActor :type Actor%20Object%20Reference) (OtherComp :type Primitive%20Component%20Object%20Reference) (OtherBodyIndex :type Integer) (bFromSweep :type Boolean) (SweepResult :type Hit%20Result%20Structure%20%28by%20ref%29))
  (if (!= OtherActor self)
    (bind _asbp_captain (Utilities|Casting|CastToBP_Captain OtherActor))
    ;[1 1 1] Custom AIC w/ interface to SetAttackTarget
    (bind _asaic_shark (Utilities|Casting|CastToAIC_Shark (AI|GetAIController self)))
    (Default|SetAttackTarget _asaic_shark _asbp_captain)))

(event EventBeginPlay
  (Development|SetHiddeninGame (Variables|Default|GetAggroSphere) false false))

(event Collision|EventActorBeginOverlap
  (params (OtherActor :type Actor%20Object%20Reference)))

(event EventTick
  (params (DeltaSeconds :type Float%20%28single-precision%29))
  (Rendering|Components|TextRender|SetText (Variables|Default|GetDebugHP) (Utilities|Text|ToText(Integer) (Variables|/Script/ActionPlatformer2D3D.APCombatComponent|GetCurrentHealth (Variables|Default|GetCombatComponent))))
  (Rendering|Components|TextRender|SetText (Variables|Default|GetHitBoxActive) (Utilities|Text|ToText(Boolean) (Utilities|Enum|Equal(Enum) "QueryOnly" (Collision|GetCollisionEnabled (Variables|Default|GetAttackHitBox))))))

(fn ConstructionScript)